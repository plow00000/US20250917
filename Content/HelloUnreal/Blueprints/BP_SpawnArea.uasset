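; BP_SpawnArea is a trigger volume that spawns BP_Rock actors inside itself when the player character type enters it.
; Each Box begin-overlap by a BP_ThirdPersonCharacter spawns one rock at a random point within the box's scaled extents.
; A Count variable increments with each spawn and stops spawning once it reaches ten.
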(event `self.Box.OnComponentBeginOverlap`
  (params (OverlappedComponent :type "PrimitiveComponent Object Reference") (OtherActor :type "Actor Object Reference") (OtherComp :type "PrimitiveComponent Object Reference") (OtherBodyIndex :type Integer) (bFromSweep :type Boolean) (SweepResult :type "HitResult Structure (by ref)"))
  (bind _box (`self.Box`))
  (cast `/Game/ThirdPerson/Blueprints/BP_ThirdPersonCharacter` OtherActor)
  (if (< (`self.Count`) 10)
    (`|SpawnActorFromClass` "/Game/HelloUnreal/Blueprints/BP_Rock.BP_Rock_C" (`KismetMathLibrary.MakeTransform` (`KismetMathLibrary.RandomPointInBoundingBox` (`SceneComponent.K2_GetComponentLocation` _box) (`BoxComponent.GetScaledBoxExtent` _box))) "Undefined" "MultiplyWithRoot" null null)
    (set `self.Count` (+ (`self.Count`) 1))))

(fn `UserConstructionScript`)