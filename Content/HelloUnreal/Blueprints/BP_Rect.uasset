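; BP_Rect is a Blueprint that moves its AAA component endlessly around a square path in the relative X-Z plane.
; Each Tick, a MovingState switch cycles Up, Left, Down and Right, stepping one coordinate until it reaches its bound, then changing state.
; Steps are fixed per frame, with no delta-time scaling.
; An older left-right ping-pong driven by IsMovingRight remains in the graph but never runs.
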(event `self.ReceiveTick`
  (params (DeltaSeconds :type "Float (single-precision)"))
  (bind _locationz (`self.LocationZ`))
  (bind _locationz_2 (`self.LocationZ`))
  (bind _locationx (`self.LocationX`))
  (bind _locationx_2 (`self.LocationX`))
  (switch `/Game/HelloUnreal/Blueprints/EN_MoveType` (`self.MovingState`)
    (:`NewEnumerator0`
      (if (>= _locationz 500.0)
        (set `self.MovingState` "NewEnumerator1")
        (else
          (set `self.LocationZ` (+ _locationz 5.0))
          (`SceneComponent.K2_SetRelativeLocation` (`self.AAA`) (`KismetMathLibrary.MakeVector` (`self.LocationX`) 0.0 (`self.LocationZ`)) false false :!label _label))))
    (:`NewEnumerator1`
      (if (<= _locationx 0.0)
        (set `self.MovingState` "NewEnumerator2")
        (else
          (set `self.LocationX` (+ _locationx -5.0))
          (goto _label))))
    (:`NewEnumerator2`
      (if (<= _locationz_2 0.0)
        (set `self.MovingState` "NewEnumerator3")
        (else
          (set `self.LocationZ` (+ _locationz_2 -5.0))
          (goto _label))))
    (:`NewEnumerator3`
      (if (>= _locationx_2 500.0)
        (set `self.MovingState` "NewEnumerator0")
        (else
          (set `self.LocationX` (+ _locationx_2 5.0))
          (goto _label))))))

(fn `UserConstructionScript`)